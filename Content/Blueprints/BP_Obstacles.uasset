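; Configurable obstacle actor that applies a chosen mesh, material and transform at BeginPlay, then animates its Model component.
; Each Tick runs Movement, Rotation and Scaling, each gated by its own toggle and scaled by Speed and delta time.
; Movement and Scaling step at constant speed through looping arrays of relative targets, advancing within a tolerance, with scaling using Speed/100.
; Rotation spins continuously by adding RotateDirection to the relative rotation.
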(event Custom|SetLocationObstacles
  (Transformation|SetRelativeLocation (Variables|Default|GetModel) (Variables|Default|GetcurrentLocation) false false))

(event Custom|SetRotate%20Obstacles
  (Transformation|SetRelativeRotation (Variables|Default|GetModel) (Variables|Default|GetcurrentRotate) false false))

(event Custom|SetScale%20Obstacles
  (Transformation|SetRelativeScale3D (Variables|Default|GetModel) (Variables|Default|GetcurrentScale)))

(event EventBeginPlay
  (CallFunction|SetMesh))

(event Collision|EventActorBeginOverlap
  (params (OtherActor :type Actor%20Object%20Reference)))

(event EventTick
  (params (DeltaSeconds :type Float%20%28single-precision%29))
  (Utilities|FlowControl|Sequence
    (:then_0
      (CallFunction|Movement))
    (:then_1
      (CallFunction|Rotation))
    (:then_2
      (CallFunction|Scaling))))

(fn ConstructionScript)

(fn Movement
  (bind _model (Variables|Default|GetModel))
  (bind _relativelocation (Variables|/Script/Engine.SceneComponent|GetRelativeLocation _model))
  (if (Variables|Default|GetMoving)
    (if (|(((x<=a)&&(y<=a))&&(z<=a)) (.X (Math|Vector|BreakVector (Math|Vector|VectorGetAbs (|(target-Self) (Utilities|Array|Get(acopy) (Variables|Default|GetTargetsToMove) (Math|Conversions|ToInteger(Byte) (Variables|Default|GettargetsIndex))) _relativelocation)))) (.Y (Math|Vector|BreakVector (Math|Vector|VectorGetAbs (|(target-Self) (Utilities|Array|Get(acopy) (Variables|Default|GetTargetsToMove) (Math|Conversions|ToInteger(Byte) (Variables|Default|GettargetsIndex))) _relativelocation)))) (.Z (Math|Vector|BreakVector (Math|Vector|VectorGetAbs (|(target-Self) (Utilities|Array|Get(acopy) (Variables|Default|GetTargetsToMove) (Math|Conversions|ToInteger(Byte) (Variables|Default|GettargetsIndex))) _relativelocation)))) 5.0)
      (if (|(({0DF72DD1-4924-D325-1268-4F8EFE8CA470}+1)==len) (Utilities|Array|Length (Variables|Default|GetTargetsToMove)))
        (Variables|Default|SettargetsIndex 0)
        (else
          (Variables|Default|SettargetsIndex (Math|Conversions|ToByte(Integer) (|({0DF72DD1-4924-D325-1268-4F8EFE8CA470}+1))))))
      (else
        (Variables|Default|SetcurrentLocation (|(Self+((Normalize*DeltaSeconds)*{AB8CA857-4FE2-755D-4381-948A8AAD8286})) (Math|Vector|Normalize (|(target-Self) (Utilities|Array|Get(acopy) (Variables|Default|GetTargetsToMove) (Math|Conversions|ToInteger(Byte) (Variables|Default|GettargetsIndex))) _relativelocation)) _relativelocation (Utilities|Time|GetWorldDeltaSeconds)))
        (CallFunction|SetLocationObstacles)
        (return)))))

(fn SetMesh
  (bind _model (Variables|Default|GetModel))
  (Components|StaticMesh|SetStaticMesh _model (Variables|Default|GetMesh))
  (Rendering|Material|SetMaterial _model 0 (Variables|Default|GetMesh_Material))
  (Class|SceneComponent|AddLocalTransform _model (Variables|Default|GetMesh_Transform) false false))

(fn Rotation
  (bind _returnvalue (Utilities|Time|GetWorldDeltaSeconds))
  (bind _model (Variables|Default|GetModel))
  (bind _rotatedirection (Variables|Default|GetrotateDirection))
  (bind _returnvalue_2 (|((rd*{AB8CA857-4FE2-755D-4381-948A8AAD8286})*DeltaSeconds) _rotatedirection _returnvalue))
  (bind _relativerotation (Variables|/Script/Engine.SceneComponent|GetRelativeRotation _model))
  (bind (_roll _pitch _yaw) (Math|Rotator|BreakRotator _relativerotation))
  (bind (_x _y _z) (Math|Vector|BreakVector _returnvalue_2))
  (bind _returnvalue_3 (|(vector((x1+x2),(y1+y2),(z1+z2))) _roll _x _pitch _y _yaw _z))
  (bind (_x_2 _y_2 _z_2) (Math|Vector|BreakVector _returnvalue_3))
  (if (Variables|Default|GetRotate)
    (Variables|Default|SetcurrentRotate (Math|Rotator|MakeRotator _x_2 _y_2 _z_2))
    (CallFunction|SetRotateObstacles)))

(fn Scaling
  (bind _model (Variables|Default|GetModel))
  (bind _relativescale3d (Variables|/Script/Engine.SceneComponent|GetRelativeScale3D _model))
  (if (Variables|Default|GetScale)
    (if (|(((x<=a)&&(y<=a))&&(z<=a)) (.X (Math|Vector|BreakVector (Math|Vector|VectorGetAbs (|(target-Self) (Utilities|Array|Get(acopy) (Variables|Default|GetTargetsScale) (Math|Conversions|ToInteger(Byte) (Variables|Default|GettargetsScaleIndex))) _relativescale3d)))) (.Y (Math|Vector|BreakVector (Math|Vector|VectorGetAbs (|(target-Self) (Utilities|Array|Get(acopy) (Variables|Default|GetTargetsScale) (Math|Conversions|ToInteger(Byte) (Variables|Default|GettargetsScaleIndex))) _relativescale3d)))) (.Z (Math|Vector|BreakVector (Math|Vector|VectorGetAbs (|(target-Self) (Utilities|Array|Get(acopy) (Variables|Default|GetTargetsScale) (Math|Conversions|ToInteger(Byte) (Variables|Default|GettargetsScaleIndex))) _relativescale3d)))) 0.1)
      (if (|(({CF2C3E9A-494A-7C72-4DF0-60A063F6FD73}+1)==len) (Utilities|Array|Length (Variables|Default|GetTargetsScale)))
        (Variables|Default|SettargetsScaleIndex 0)
        (else
          (Variables|Default|SettargetsScaleIndex (Math|Conversions|ToByte(Integer) (|({CF2C3E9A-494A-7C72-4DF0-60A063F6FD73}+1))))))
      (else
        (Variables|Default|SetcurrentScale (|(Self+((Normalize*DeltaSeconds)*({AB8CA857-4FE2-755D-4381-948A8AAD8286}/100))) (Math|Vector|Normalize (|(target-Self) (Utilities|Array|Get(acopy) (Variables|Default|GetTargetsScale) (Math|Conversions|ToInteger(Byte) (Variables|Default|GettargetsScaleIndex))) _relativescale3d)) _relativescale3d (Utilities|Time|GetWorldDeltaSeconds)))
        (CallFunction|SetScaleObstacles)))))