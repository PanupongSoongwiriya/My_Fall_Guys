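; Actor that moves its Cube back and forth along a Bézier curve defined by an array of control points.
; Tick runs a timer up and down over the Time duration, flipping Switch at each end and normalizing it into the curve parameter.
; Point3 sums control points weighted by Bernstein polynomials, built from factorial-based binomial coefficients.
; The result offsets the Cube from its starting relative location, with an optional debug line.
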(event Custom|CreateBezierCurve
  (bind _startline (Variables|Default|GetstartLine))
  ;[1 1 1] Bézier Curve
  (bind _newparam (CallFunction|Point3 (|(({1A604124-45A3-49EA-4603-CAB5C4310FE5}-{EAC25C5E-4A97-E3C8-4057-6CB0967BD357})/{1A604124-45A3-49EA-4603-CAB5C4310FE5}))))
  (Utilities|FlowControl|Sequence
    (:then_0
      (if (Variables|Default|GetshowLine)
        (Rendering|Debug|DrawDebugLine _startline (+ _startline _newparam) "(R=0.000000,G=1.000000,B=0.000000,A=1.000000)" (Variables|Default|Gettime) 1.0)))
    (:then_1
      (Transformation|SetRelativeLocation (Variables|Default|GetCube) (+ (Variables|Default|GetstartVector) _newparam) false false))))

(event Custom|SetTime
  (CallFunction|CreateBezierCurve))

(event EventBeginPlay
  ;[1 1 1] SetStartVector
  (Variables|Default|SetstartLine (Transformation|GetActorLocation))
  (Variables|Default|SetstartVector (Variables|/Script/Engine.SceneComponent|GetRelativeLocation (Variables|Default|GetCube)))
  (Variables|Default|SetcurrentTime (Variables|Default|Gettime)))

(event Collision|EventActorBeginOverlap
  (params (OtherActor :type Actor%20Object%20Reference)))

(event EventTick
  (params (DeltaSeconds :type Float%20%28single-precision%29))
  (if (Variables|Default|Getswitch)
    ;[1 1 1] Go Back
    (Variables|Default|SetcurrentTime (|({EAC25C5E-4A97-E3C8-4057-6CB0967BD357}+d) DeltaSeconds))
    (if (|({1A604124-45A3-49EA-4603-CAB5C4310FE5}>{EAC25C5E-4A97-E3C8-4057-6CB0967BD357}))
      (CallFunction|SetTime :!label _label)
      (else
        (Variables|Default|SetcurrentTime (Variables|Default|Gettime))
        (Variables|Default|Setswitch false)))
    (else
      ;[1 1 1] Go Ahead
      (Variables|Default|SetcurrentTime (|({EAC25C5E-4A97-E3C8-4057-6CB0967BD357}-d) DeltaSeconds))
      (if (|(0<{EAC25C5E-4A97-E3C8-4057-6CB0967BD357}))
        (goto _label)
        (else
          (Variables|Default|SetcurrentTime 0.0)
          (Variables|Default|Setswitch true))))))

(fn ConstructionScript)

(fn NI
  (params (n :type Integer) (i :type Integer))
  (bind _result (CallFunction|FindFactorial n))
  (LocalVariables|SetFactorial_n _result)
  (bind _result_2 (CallFunction|FindFactorial i))
  (LocalVariables|SetFactorial_i _result_2)
  (bind _result_3 (CallFunction|FindFactorial (|(n-i) n i)))
  (LocalVariables|SetFactorial_ni _result_3)
  (return (Math|Conversions|ToFloat(Integer) (|({EFACA315-4D22-D8F1-3F83-078BFF169692}/({087D86F1-45F5-37C2-B8CD-ED803B409025}*{DA660520-438F-E607-FA9A-78AB4B30A4AD}))))))

(fn FindFactorial
  (params (n :type Integer))
  (for _index (range 1 n)
    (LocalVariables|Setans (|({9F660DB5-4B6F-6DE2-68B1-0A955FD1D7E6}*i) _index)))
  (return (LocalVariables|Getans)))

(fn Bernstein
  (params (n :type Integer) (i :type Integer) (timr :type Float%20%28double-precision%29))
  (bind _return (CallFunction|NI n i))
  (return (* _return (|((pow(t,i))*(pow((1-t),(n-i)))) (Math|Conversions|ToFloat(Integer) n) (Math|Conversions|ToFloat(Integer) i) timr))))

(fn Point3
  (params (time :type Float%20%28double-precision%29))
  (bind _controlpoints (Variables|Default|GetcontrolPoints))
  (if (<= time 0.0)
    (return (Utilities|Array|Get(acopy) (Variables|Default|GetcontrolPoints)))
    (elif (>= time 1.0)
      (return (Utilities|Array|Get(acopy) _controlpoints (- (Utilities|Array|Length _controlpoints) 1)))
      (else
        (for (_array_element _array_index) (Variables|Default|GetcontrolPoints)
          (bind _result (CallFunction|Bernstein (|(a-1) (Utilities|Array|Length (Variables|Default|GetcontrolPoints))) _array_index time))
          (LocalVariables|Setp (+ (* _array_element _result) (LocalVariables|Getp))))
        (return (LocalVariables|Getp))))))