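; Checkpoint actor that records the player's progress through a level by saving its own location on the player.
; It overrides the parent's OverlappingEffects function, calls the parent version, then uses a math expression to compare the player's CheckPointIndex with its own Index.
; Only a higher-indexed checkpoint overwrites the player's CheckPointLocation and CheckPointIndex, so earlier checkpoints cannot roll progress back.
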(event EventBeginPlay
  (|CallParentFunction) ; This node is disabled and will not be called.\nDrag off pins to build functionality.
)

(event Collision|EventActorBeginOverlap
  (params (OtherActor :type Actor%20Object%20Reference))
  (|CallParentFunction OtherActor) ; This node is disabled and will not be called.\nDrag off pins to build functionality.
)

(event EventTick
  (params (DeltaSeconds :type Float%20%28single-precision%29))
  (|CallParentFunction DeltaSeconds) ; This node is disabled and will not be called.\nDrag off pins to build functionality.
)

(fn ConstructionScript
  (|CallParentFunction))

(fn OverlappingEffects
  (params (Player :type BP%20Third%20Person%20Character%20Object%20Reference))
  (|CallParentFunction Player)
  (if (|(cpi<{48F51050-449B-1AFD-7683-80B9CFA8C2C9}) (Variables|/Game/ThirdPerson/Blueprints/BP_ThirdPersonCharacter.BP_ThirdPersonCharacter_C|GetcheckPointIndex Player))
    (Variables|/Game/ThirdPerson/Blueprints/BP_ThirdPersonCharacter.BP_ThirdPersonCharacter_C|SetcheckPointLocation Player (Transformation|GetActorLocation))
    (Variables|/Game/ThirdPerson/Blueprints/BP_ThirdPersonCharacter.BP_ThirdPersonCharacter_C|SetcheckPointIndex Player (Variables|Default|GetIndex))))