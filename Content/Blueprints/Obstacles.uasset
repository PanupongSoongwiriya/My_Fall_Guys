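; Configurable obstacle actor that animates a static mesh by moving, rotating and scaling it, each behind its own toggle.
; BeginPlay applies the chosen mesh, material and transform offset, then Tick runs the three motions scaled by delta time.
; Movement and scaling read Direction, Min and Max from maps; crossing a bound stops, reverses or resets the mesh transform, per behaviour enum.
; Rotation spins the whole actor continuously, while movement and scaling affect only the mesh component.
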(event EventBeginPlay
  (CallFunction|SetMesh))

(event Collision|EventActorBeginOverlap
  (params (OtherActor :type Actor%20Object%20Reference)))

(event EventTick
  (params (DeltaSeconds :type Float%20%28single-precision%29))
  (Variables|Default|SetDeltaTime DeltaSeconds)
  (CallFunction|Movement)
  (CallFunction|Rotation)
  (CallFunction|Scaling))

(fn ConstructionScript)

(fn SetMesh
  (bind _staticmesh (Variables|Default|GetStaticMesh))
  (Components|StaticMesh|SetStaticMesh _staticmesh (Variables|Default|GetMesh))
  (Rendering|Material|SetMaterial _staticmesh 0 (Variables|Default|GetMesh_Material))
  (Class|SceneComponent|AddLocalTransform _staticmesh (Variables|Default|GetMesh_Transform) false false))

(fn Movement
  (bind _move_behaviour (Variables|Default|GetMove%20Behaviour))
  (bind _movedata (Variables|Default|GetMoveData))
  (bind _movedata_2 (Variables|Default|GetMoveData))
  (bind _staticmesh (Variables|Default|GetStaticMesh))
  (bind _staticmesh_2 (Variables|Default|GetStaticMesh))
  (bind _movedata_3 (Variables|Default|GetMoveData))
  (bind (_value _returnvalue) (Utilities|Map|Find _movedata_3 "Direction"))
  (bind (_value_2 _returnvalue_2) (Utilities|Map|Find _movedata "Max"))
  (bind _returnvalue_3 (Transformation|GetRelativeTransform _staticmesh_2))
  (bind (_value_3 _returnvalue_4) (Utilities|Map|Find _movedata_2 "Min"))
  (bind _returnvalue_5 (Transformation|GetRelativeTransform _staticmesh))
  (bind (_x _y _z) (Math|Vector|BreakVector _value_3))
  (bind _location (Math|Transform|BreakTransform _returnvalue_3))
  (bind (_x_2 _y_2 _z_2) (Math|Vector|BreakVector _value_2))
  (bind _location_2 (Math|Transform|BreakTransform _returnvalue_5))
  (bind (_x_3 _y_3 _z_3) (Math|Vector|BreakVector _location_2))
  (bind (_x_4 _y_4 _z_4) (Math|Vector|BreakVector _location))
  (if (Variables|Default|GetMoving)
    ;[1 0.56 0] Movemonet
    (if _returnvalue
      (Transformation|AddLocalOffset (Variables|Default|GetStaticMesh) (* _value (* (Variables|Default|GetDeltaTime) (Variables|Default|GetInverseDirectionMove))) false false)
      (if (> 0 (Variables|Default|GetInverseDirectionMove))
        ;[0 1 0.107] CheckMin
        (if _returnvalue_4
          (if (Math|Boolean|ORBoolean (> _x _x_3) (> _y _y_3) (> _z _z_3))
            ;[1 1 1] Behaviour
            (if (Utilities|Enum|Equal(Enum) _move_behaviour "NewEnumerator0") :!label _label
              (Variables|Default|SetInverseDirectionMove 0)
              (elif (Utilities|Enum|Equal(Enum) _move_behaviour "NewEnumerator2")
                (Variables|Default|SetInverseDirectionMove (* -1 (Variables|Default|GetInverseDirectionMove)))
                (else
                  (Transformation|SetRelativeTransform (Variables|Default|GetStaticMesh) (Variables|Default|GetMesh_Transform) false false))))))
        (else
          ;[1 0 0] CheckMax
          (if _returnvalue_2
            (if (Math|Boolean|ORBoolean (< _x_2 _x_4) (< _y_2 _y_4) (< _z_2 _z_4))
              (goto _label))))))))

(fn Rotation
  (bind _ratatedata (Variables|Default|GetRatateData))
  (bind _deltatime (Variables|Default|GetDeltaTime))
  (bind _returnvalue (* _ratatedata _deltatime))
  (bind (_x _y _z) (Math|Vector|BreakVector _returnvalue))
  (if (Variables|Default|GetRotate)
    ;[1 0.56 0] Rotation
    (Transformation|AddActorLocalRotation (Math|Rotator|MakeRotator _x _y _z) false false)))

(fn Scaling
  (bind _scaledata (Variables|Default|GetScaleData))
  (bind _scaledata_2 (Variables|Default|GetScaleData))
  (bind _scaledata_3 (Variables|Default|GetScaleData))
  (bind _staticmesh (Variables|Default|GetStaticMesh))
  (bind _scale_behaviour (Variables|Default|GetScale%20Behaviour))
  (bind _staticmesh_2 (Variables|Default|GetStaticMesh))
  (bind (_value _returnvalue) (Utilities|Map|Find _scaledata_2 "Direction"))
  (bind (_value_2 _returnvalue_2) (Utilities|Map|Find _scaledata "Max"))
  (bind _returnvalue_3 (Transformation|GetRelativeTransform _staticmesh))
  (bind (_value_3 _returnvalue_4) (Utilities|Map|Find _scaledata_3 "Min"))
  (bind _returnvalue_5 (Transformation|GetRelativeTransform _staticmesh_2))
  (bind (_x _y _z) (Math|Vector|BreakVector _value_3))
  (bind _scale (Math|Transform|BreakTransform _returnvalue_3))
  (bind (_x_2 _y_2 _z_2) (Math|Vector|BreakVector _value_2))
  (bind _scale_2 (Math|Transform|BreakTransform _returnvalue_5))
  (bind (_x_3 _y_3 _z_3) (Math|Vector|BreakVector _scale_2))
  (bind (_x_4 _y_4 _z_4) (Math|Vector|BreakVector _scale))
  (if (Variables|Default|GetScale)
    ;[1 1 1] Scaling
    (if _returnvalue
      (Transformation|SetRelativeScale3D (Variables|Default|GetStaticMesh) (+ (* _value (* (Variables|Default|GetDeltaTime) (Variables|Default|GetInverseDirectionScale))) (.Scale (Math|Transform|BreakTransform (Transformation|GetRelativeTransform (Variables|Default|GetStaticMesh))))))
      (if (> 0 (Variables|Default|GetInverseDirectionScale))
        ;[0 1 0.107] CheckMin
        (if _returnvalue_4
          (if (Math|Boolean|ORBoolean (> _x _x_3) (> _y _y_3) (> _z _z_3))
            ;[1 1 1] Behaviour
            (if (Utilities|Enum|Equal(Enum) _scale_behaviour "NewEnumerator0") :!label _label
              (Variables|Default|SetInverseDirectionScale 0)
              (elif (Utilities|Enum|Equal(Enum) _scale_behaviour "NewEnumerator2")
                (Variables|Default|SetInverseDirectionScale (* -1 (Variables|Default|GetInverseDirectionScale)))
                (else
                  (Transformation|SetRelativeTransform (Variables|Default|GetStaticMesh) (Variables|Default|GetMesh_Transform) false false))))))
        (else
          ;[1 0 0] CheckMax
          (if _returnvalue_2
            (if (Math|Boolean|ORBoolean (< _x_2 _x_4) (< _y_2 _y_4) (< _z_2 _z_4))
              (goto _label))))))))