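; BP_FinishLine is the race finish actor that declares the first player to reach it the winner and restarts the game.
; Its override of the parent's OverlappingEffects latches PlayerEnter, prints the player's display name as winner in green, then immediately calls RestartGame on the GameMode.
; A countdown-delayed restart remains in the event graph but is disconnected from Tick and never runs.
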(event EventBeginPlay
  (|CallParentFunction) ; This node is disabled and will not be called.\nDrag off pins to build functionality.
)

(event Collision|EventActorBeginOverlap
  (params (OtherActor :type Actor%20Object%20Reference))
  (|CallParentFunction OtherActor) ; This node is disabled and will not be called.\nDrag off pins to build functionality.
)

(event EventTick
  (params (DeltaSeconds :type Float%20%28single-precision%29)))

(fn ConstructionScript
  (|CallParentFunction))

(fn OverlappingEffects
  (params (Player :type BP%20Third%20Person%20Character%20Object%20Reference))
  (|CallParentFunction Player)
  ;[1 1 1] Print The Winner name
  (if (not (Variables|Default|GetplayerEnter))
    (Variables|Default|SetplayerEnter true)
    (Development|PrintString (Utilities|String|Append (Utilities|GetDisplayName Player) "Winner!!!") true true "(R=0.000000,G=1.000000,B=0.000000,A=1.000000)" 15.0)
    ;[1 1 1] RestartGame
    (bind _asgame_mode (Utilities|Casting|CastToGameMode (Game|GetGameMode)))
    (Class|GameMode|RestartGame _asgame_mode)))