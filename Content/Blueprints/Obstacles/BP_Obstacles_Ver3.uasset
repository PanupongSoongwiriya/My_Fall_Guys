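; A moving obstacle actor that shifts its static mesh through a looping array of target locations while blending rotation and scale toward single targets.
; Tick counts Time down into a clamped 0–1 Alpha, then calls ProcessOnServer, which relays to an all-player event that lerps the relative transform.
; At full Alpha, the reached location becomes the next start, the index advances or wraps, and the timer resets.
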(event Custom|Process%20On%20Server
  (CallFunction|SetTransformatAllPlayer))

(event Custom|Set%20transform%20at%20all%20player
  (bind _alpha (Variables|Default|Getalpha))
  ;[1 1 1] Change Transform
  (Development|PrintString (Utilities|String|ToString(Float) _alpha) true true "(R=0.000000,G=1.000000,B=0.125318,A=1.000000)" 99.0)
  (Transformation|SetRelativeTransform (Variables|Default|GetStaticMesh) (Math|Transform|MakeTransform (Math|Vector|Lerp(Vector) (Variables|PropertyLocation|GetcurrentLocation) (Utilities|Array|Get(acopy) (Variables|PropertyLocation|GetTargetLocation) (Math|Conversions|ToInteger(Byte) (Variables|PropertyLocation|GettargetsIndex))) _alpha) (Math|Rotator|Lerp(Rotator) (Variables|PropertyRotate|GetcurrentRotate) (Variables|PropertyRotate|GetTargetRotation) _alpha) (Math|Vector|Lerp(Vector) (Variables|PropertyScale|GetcurrentScale) (Variables|PropertyScale|GetTargetScale) _alpha)) false false))

(event EventBeginPlay
  (bind _staticmesh (Variables|Default|GetStaticMesh))
  (bind _returnvalue (Transformation|GetRelativeTransform _staticmesh))
  (bind (_location _rotation _scale) (Math|Transform|BreakTransform _returnvalue))
  ;[1 1 1] Set Default
  (Variables|PropertyLocation|SetcurrentLocation _location)
  (Variables|PropertyRotate|SetcurrentRotate _rotation)
  (Variables|PropertyScale|SetcurrentScale _scale)
  (Variables|Default|SetdefaultTime (Variables|Default|GetTime)))

(event Collision|EventActorBeginOverlap
  (params (OtherActor :type Actor%20Object%20Reference)))

(event EventTick
  (params (DeltaSeconds :type Float%20%28single-precision%29))
  (bind _targetlocation (Variables|PropertyLocation|GetTargetLocation))
  (Utilities|FlowControl|Sequence
    (:then_0
      ;[1 1 1] Set Alpha
      (if (|({FB74625F-439F-FED5-06FF-358C8983F7B6}>0))
        (Variables|Default|SetTime (|({FB74625F-439F-FED5-06FF-358C8983F7B6}-delta) DeltaSeconds))
        (Variables|Default|Setalpha (* (|(({FB74625F-439F-FED5-06FF-358C8983F7B6}-{7A7B6031-47F9-CDCE-F13B-179F1FEAD982})/{7A7B6031-47F9-CDCE-F13B-179F1FEAD982})) -1.0))
        (Variables|Default|Setalpha (|(Min((Max(0,a)),1)) (Variables|Default|Getalpha)))
        (CallFunction|ProcessonServer)))
    (:then_1
      ;[1 1 1] Change Index when alpha ==1
      (if (|({5D82957A-4568-117D-2A59-2D99EB222223}==1))
        (Variables|PropertyLocation|SetcurrentLocation (Utilities|Array|Get(acopy) _targetlocation (Math|Conversions|ToInteger(Byte) (Variables|PropertyLocation|GettargetsIndex))))
        (if (|(({DDDD98CD-4CC3-8773-4BED-74AD0794A181}+1)==len) (Utilities|Array|Length _targetlocation))
          (Variables|PropertyLocation|SettargetsIndex 0)
          (else
            (Variables|PropertyLocation|SettargetsIndex (Math|Conversions|ToByte(Integer) (|({DDDD98CD-4CC3-8773-4BED-74AD0794A181}+1))))))
        (Variables|Default|SetTime (Variables|Default|GetdefaultTime))))))

(fn ConstructionScript)