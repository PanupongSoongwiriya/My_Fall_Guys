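; Obstacle actor that can move, rotate and scale on Tick, with each behavior toggled independently.
; Movement and scaling step the Model component at constant speed through looping target arrays, advancing once within a per-axis tolerance.
; Rotation spins either the Model or the whole actor continuously, depending on RotationType.
; Each new transform goes through CalculateNew events into Set events intended to apply it on server and clients.
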(event Custom|Set%20Location%20Obstacles
  ;[1 1 1] Set location both server and clients
  (Transformation|SetRelativeLocation (Variables|Default|GetModel) (Variables|Default|GetcurrentLocation) false false))

(event Custom|Calculate%20New%20Location
  (CallFunction|SetLocationObstacles))

(event Custom|Set%20Rotate%20Obstacles
  (bind _currentrotate (Variables|Default|GetcurrentRotate))
  ;[1 1 1] Set rotation both server and clients
  (if (Utilities|Enum|Equal(Enum) (Variables|Default|GetRotationType) "NewEnumerator1")
    (Transformation|SetRelativeRotation (Variables|Default|GetModel) _currentrotate false false)
    (else
      (Transformation|SetActorRotation _currentrotate))))

(event Custom|Calculate%20New%20Rotate
  (CallFunction|SetRotateObstacles))

(event Custom|Calculate%20New%20Scale
  (CallFunction|SetScaleObstacles))

(event Custom|Set%20Scale%20Obstacles
  ;[1 1 1] Set scale both server and clients
  (Transformation|SetRelativeScale3D (Variables|Default|GetModel) (Variables|Default|GetcurrentScale)))

(event EventBeginPlay)

(event Collision|EventActorBeginOverlap
  (params (OtherActor :type Actor%20Object%20Reference)))

(event EventTick
  (params (DeltaSeconds :type Float%20%28single-precision%29))
  (Utilities|FlowControl|Sequence
    (:then_0
      (CallFunction|Movement))
    (:then_1
      (CallFunction|Rotation))
    (:then_2
      (CallFunction|Scaling))))

(fn ConstructionScript)

(fn Movement
  (bind _model (Variables|Default|GetModel))
  (bind _relativelocation (Variables|/Script/Engine.SceneComponent|GetRelativeLocation _model))
  (if (Variables|Default|GetMoving)
    (if (|(((x<=a)&&(y<=a))&&(z<=a)) (.X (Math|Vector|BreakVector (Math|Vector|VectorGetAbs (|(target-Self) (Utilities|Array|Get(acopy) (Variables|Default|GetTargetsToMove) (Math|Conversions|ToInteger(Byte) (Variables|Default|GettargetsIndex))) _relativelocation)))) (.Y (Math|Vector|BreakVector (Math|Vector|VectorGetAbs (|(target-Self) (Utilities|Array|Get(acopy) (Variables|Default|GetTargetsToMove) (Math|Conversions|ToInteger(Byte) (Variables|Default|GettargetsIndex))) _relativelocation)))) (.Z (Math|Vector|BreakVector (Math|Vector|VectorGetAbs (|(target-Self) (Utilities|Array|Get(acopy) (Variables|Default|GetTargetsToMove) (Math|Conversions|ToInteger(Byte) (Variables|Default|GettargetsIndex))) _relativelocation)))) (|({AB8CA857-4FE2-755D-4381-948A8AAD8286}/100)))
      ;[1 1 1] Set Next Target
      (if (|(({0DF72DD1-4924-D325-1268-4F8EFE8CA470}+1)==len) (Utilities|Array|Length (Variables|Default|GetTargetsToMove)))
        (Variables|Default|SettargetsIndex 0)
        (else
          (Variables|Default|SettargetsIndex (Math|Conversions|ToByte(Integer) (|({0DF72DD1-4924-D325-1268-4F8EFE8CA470}+1))))))
      (else
        (Variables|Default|SetcurrentLocation (|(Self+((Normalize*DeltaSeconds)*{AB8CA857-4FE2-755D-4381-948A8AAD8286})) (Math|Vector|Normalize (|(target-Self) (Utilities|Array|Get(acopy) (Variables|Default|GetTargetsToMove) (Math|Conversions|ToInteger(Byte) (Variables|Default|GettargetsIndex))) _relativelocation)) _relativelocation (Utilities|Time|GetWorldDeltaSeconds)))
        (CallFunction|CalculateNewLocation)))))

(fn Rotation
  (bind _returnvalue (Utilities|Time|GetWorldDeltaSeconds))
  (bind _rotatedirection (Variables|Default|GetrotateDirection))
  (bind _returnvalue_2 (|((rd*{AB8CA857-4FE2-755D-4381-948A8AAD8286})*DeltaSeconds) _rotatedirection _returnvalue))
  (bind (_x _y _z) (Math|Vector|BreakVector _returnvalue_2))
  (if (Variables|Default|GetRotate)
    ;[1 1 1] Check the target you want to rotate.
    (if (Utilities|Enum|Equal(Enum) (Variables|Default|GetRotationType) "NewEnumerator1")
      (Variables|Default|SettargetRotate (Variables|/Script/Engine.SceneComponent|GetRelativeRotation (Variables|Default|GetModel)))
      (else
        (Variables|Default|SettargetRotate (Transformation|GetActorRotation))))
    (Variables|Default|SetcurrentRotate (Math|Rotator|MakeRotator (.X (Math|Vector|BreakVector (|(vector((x1+x2),(y1+y2),(z1+z2))) (.Roll (Math|Rotator|BreakRotator (Variables|Default|GettargetRotate))) _x (.Pitch (Math|Rotator|BreakRotator (Variables|Default|GettargetRotate))) _y (.Yaw (Math|Rotator|BreakRotator (Variables|Default|GettargetRotate))) _z))) (.Y (Math|Vector|BreakVector (|(vector((x1+x2),(y1+y2),(z1+z2))) (.Roll (Math|Rotator|BreakRotator (Variables|Default|GettargetRotate))) _x (.Pitch (Math|Rotator|BreakRotator (Variables|Default|GettargetRotate))) _y (.Yaw (Math|Rotator|BreakRotator (Variables|Default|GettargetRotate))) _z))) (.Z (Math|Vector|BreakVector (|(vector((x1+x2),(y1+y2),(z1+z2))) (.Roll (Math|Rotator|BreakRotator (Variables|Default|GettargetRotate))) _x (.Pitch (Math|Rotator|BreakRotator (Variables|Default|GettargetRotate))) _y (.Yaw (Math|Rotator|BreakRotator (Variables|Default|GettargetRotate))) _z)))))
    (CallFunction|CalculateNewRotate)))

(fn Scaling
  (bind _model (Variables|Default|GetModel))
  (bind _relativescale3d (Variables|/Script/Engine.SceneComponent|GetRelativeScale3D _model))
  (if (Variables|Default|GetScale)
    (if (|(((x<=a)&&(y<=a))&&(z<=a)) (.X (Math|Vector|BreakVector (Math|Vector|VectorGetAbs (|(target-Self) (Utilities|Array|Get(acopy) (Variables|Default|GetTargetsScale) (Math|Conversions|ToInteger(Byte) (Variables|Default|GettargetsScaleIndex))) _relativescale3d)))) (.Y (Math|Vector|BreakVector (Math|Vector|VectorGetAbs (|(target-Self) (Utilities|Array|Get(acopy) (Variables|Default|GetTargetsScale) (Math|Conversions|ToInteger(Byte) (Variables|Default|GettargetsScaleIndex))) _relativescale3d)))) (.Z (Math|Vector|BreakVector (Math|Vector|VectorGetAbs (|(target-Self) (Utilities|Array|Get(acopy) (Variables|Default|GetTargetsScale) (Math|Conversions|ToInteger(Byte) (Variables|Default|GettargetsScaleIndex))) _relativescale3d)))) 0.1)
      ;[1 1 1] Set Next Target
      (if (|(({CF2C3E9A-494A-7C72-4DF0-60A063F6FD73}+1)==len) (Utilities|Array|Length (Variables|Default|GetTargetsScale)))
        (Variables|Default|SettargetsScaleIndex 0)
        (else
          (Variables|Default|SettargetsScaleIndex (Math|Conversions|ToByte(Integer) (|({CF2C3E9A-494A-7C72-4DF0-60A063F6FD73}+1))))))
      (else
        (Variables|Default|SetcurrentScale (|(Self+((Normalize*DeltaSeconds)*({AB8CA857-4FE2-755D-4381-948A8AAD8286}/100))) (Math|Vector|Normalize (|(target-Self) (Utilities|Array|Get(acopy) (Variables|Default|GetTargetsScale) (Math|Conversions|ToInteger(Byte) (Variables|Default|GettargetsScaleIndex))) _relativescale3d)) _relativescale3d (Utilities|Time|GetWorldDeltaSeconds)))
        (CallFunction|CalculateNewScale)))))